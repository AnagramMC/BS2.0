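; Player character Arin, with a three-step sword combo, block, evade and clamped camera pitch.
; Inputs set a body state gated by numeric thresholds, and light presses advance the attack stage.
; Tick halts movement during the attack montage and, while the AnimBP's CanHit is true, damages overlapping "Enemy" actors once per window, scaled by montage section.
; Incoming damage sets HIT and knocks Arin back, while death only prints.
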(event `InputAction|LAttack`
  (params (Key :type "Key Structure" :default "AnyKey"))
  ;[1 1 1] Basic Attack Combo
  (:`Pressed`
    (if (< (`self.ArinBodyState`) 4)
      (bind _result (`/Engine/EditorBlueprintResources/StandardMacros.IncrementInt` (`self.LightAttackCounter`))
        (:`  `
          (if (> _result 2)
            (set `self.LightAttackCounter` 3))
          (set `self.ArinBodyState` "ATTACK")
          (switch `int` (`self.LightAttackCounter`)
            (:`Default`
              (set `self.ArinCurAttack` "DEFAULT" :!label _label))
            (:`0`
              (goto _label))
            (:`1`
              (set `self.ArinCurAttack` "ATTACK1"))
            (:`2`
              (set `self.ArinCurAttack` "ATTACK2"))
            (:`3`
              (set `self.ArinCurAttack` "ATTACK3")))))
      (else
        (set `self.LightAttackCounter` 0)
        (goto _label)))))

(event `InputAction|Block`
  (params (Key :type "Key Structure" :default "AnyKey"))
  (:`Pressed`
    (if (< (`self.ArinBodyState`) 5)
      (set `self.ArinBodyState` "BLOCK"))))

(event `InputAction|Evade`
  (params (Key :type "Key Structure" :default "AnyKey"))
  (:`Pressed`
    (if (< (`self.ArinBodyState`) 6)
      (set `self.ArinBodyState` "EVADE"))))

(event `self.ReceiveBeginPlay`)

(event `self.ReceiveTick`
  (params (DeltaSeconds :type "Float (single-precision)"))
  ;[1 1 1] Tick
  (if (`AnimInstance.Montage_IsPlaying` (`self.AnimInstance`) "/Game/HeavySword/Retargeted/animation/Attack1Montage.Attack1Montage")
    (`MovementComponent.StopMovementImmediately` (`self.CharacterMovement`)))
  (if (`/Game/Player/AnimBP_BSPlayer.CanHit` (`self.AnimInstance`))
    (`self.MeleeAttack`)
    (else
      (set `self.AppliedDamage` false))))

(event `InputAxis|LookUp`
  (params (AxisValue :type "Float (single-precision)"))
  (bind _returnvalue (`GameplayStatics.GetPlayerCameraManager` 0))
  ;[1 1 1] Clamp Camera Pitch
  (set `PlayerCameraManager.ViewPitchMin` -30.0 _returnvalue)
  (set `PlayerCameraManager.ViewPitchMax` 0.0 _returnvalue)
  (`self.AddControllerPitchInput` AxisValue))

(event `self.ReceiveAnyDamage`
  (params (Damage :type "Float (single-precision)") (DamageType :type "DamageType Object Reference") (InstigatedBy :type "Controller Object Reference") (DamageCauser :type "Actor Object Reference"))
  (bind _health (`self.Health`))
  ;[1 1 1] Damage Taken
  (set `self.ArinBodyState` "HIT")
  (bind _output_get (set `self.Health` (- _health Damage)))
  (if (<= _health 0.0)
    (set `self.Health` 0.0)
    (`KismetSystemLibrary.PrintString` "DEAD" true true (struct :`R` 1.0 :`A` 1.0))
    (else
      (`self.LaunchCharacter` (`KismetMathLibrary.MakeVector` (.x (* (`KismetMathLibrary.Normal` (`self.GetActorForwardVector` DamageCauser)) 100)) (.y (* (`KismetMathLibrary.Normal` (`self.GetActorForwardVector` DamageCauser)) 100))))
      (`KismetSystemLibrary.PrintString` (`KismetStringLibrary.Conv_DoubleToString` _output_get)))))

(fn `MeleeAttack`
  (bind _returnvalue (`AnimInstance.Montage_GetCurrentSection` (`self.AnimInstance`) "/Game/HeavySword/Retargeted/animation/Attack1Montage.Attack1Montage"))
  (if (not (`self.AppliedDamage`))
    (for _array_element (`PrimitiveComponent.GetOverlappingActors` (`self.HitCollider`) null)
      (if (`self.ActorHasTag` _array_element "Enemy")
        (switch `CurrentAttack` (`self.ArinCurAttack`)
          (:`ATTACK1`
            (bind _output_get (set `self.AttackDamage` 10.0 :!label _label))
            (`GameplayStatics.ApplyDamage` _array_element _output_get)
            (`self.HitEffects`)
            (`KismetSystemLibrary.PrintString` "1st Attack Damage!"))
          (:`ATTACK2`
            (if (== _returnvalue "Attack2")
              (bind _output_get_2 (set `self.AttackDamage` 20.0 :!label _label_2))
              (`GameplayStatics.ApplyDamage` _array_element _output_get_2)
              (`self.HitEffects`)
              (`KismetSystemLibrary.PrintString` "2nd Attack Damage!")
              (else
                (goto _label))))
          (:`ATTACK3`
            (if (== _returnvalue "Attack3")
              (bind _output_get_3 (set `self.AttackDamage` 30.0))
              (`GameplayStatics.ApplyDamage` _array_element _output_get_3)
              (`self.HitEffects`)
              (`KismetSystemLibrary.PrintString` "3rd Attack Damage!" true true (struct :`R` 1.0 :`G` 0.74448 :`A` 1.0))
              (else
                (goto _label_2)))))
        (set `self.AppliedDamage` true)))))

(fn `UserConstructionScript`
  (bind _asanim_bp_bsplayer (cast `/Game/Player/AnimBP_BSPlayer` (`SkeletalMeshComponent.GetAnimInstance` (`self.Mesh`))))
  (set `self.AnimInstance` _asanim_bp_bsplayer)
  (`SceneComponent.K2_AttachTo` (`self.Sword`) (`self.Mesh`) "SwordSocket" "SnapToTarget" true))