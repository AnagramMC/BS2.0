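; Behavior tree task for melee basic enemies that switches their execute state on or off.
; It copies its IsInExecute setting to the controlled BasicEnemyMelee's Execute flag.
; When turning it off, it also tells the EnemyController's Brain to change behavior to ENGAGE.
; It finishes successfully on both paths, but a failed cast leaves the task unfinished.
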(event `self.ReceiveExecute`
  (params (OwnerActor :type "Actor Object Reference"))
  (bind _returnvalue (`AIBlueprintHelperLibrary.GetAIController` OwnerActor))
  (bind _asbasic_enemy_melee (cast `BasicEnemyMelee` (`Controller.K2_GetPawn` _returnvalue))
    (:`then`
      (if (`self.IsInExecute`)
        (set `BasicEnemyMelee.Execute` true _asbasic_enemy_melee)
        (else
          (set `BasicEnemyMelee.Execute` false _asbasic_enemy_melee)
          (bind _returnvalue_2 (`AIBlueprintHelperLibrary.GetAIController` _asbasic_enemy_melee))
          (bind _asenemy_controller (cast `EnemyController` _returnvalue_2))
          (`BehaviorComponent.ChangeBehavior` (`EnemyController.Brain` _asenemy_controller) "ENGAGE")))
      (`self.FinishExecute` true))
    (:`CastFailed`
      (`KismetSystemLibrary.PrintString` "fail"))))