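; Behavior tree task for basic melee enemies that knocks the AI's controlled character back.
; On execute, it launches that character horizontally along the first player pawn's forward vector at a fixed strength, adding to existing velocity rather than overriding it.
; The direction follows where the player faces, not the relative positions of player and enemy.
; It finishes successfully at once, even when the Character cast fails and prints a debug message.
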(event `self.ReceiveExecute`
  (params (OwnerActor :type "Actor Object Reference"))
  (bind _returnvalue (`AIBlueprintHelperLibrary.GetAIController` OwnerActor))
  (bind _ascharacter (cast `Character` (`Controller.K2_GetPawn` _returnvalue))
    (:`then`
      (`Character.LaunchCharacter` _ascharacter (`KismetMathLibrary.MakeVector` (.x (* (`KismetMathLibrary.Normal` (`Actor.GetActorForwardVector` (`GameplayStatics.GetPlayerPawn` 0))) 1000)) (.y (* (`KismetMathLibrary.Normal` (`Actor.GetActorForwardVector` (`GameplayStatics.GetPlayerPawn` 0))) 1000))) false false)
      (`self.FinishExecute` true))
    (:`CastFailed`
      (`KismetSystemLibrary.PrintString` "Fail")
      (`self.FinishExecute` true))))