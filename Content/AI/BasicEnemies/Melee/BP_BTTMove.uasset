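; Behavior tree move task for melee enemies that sends the pawn to a blackboard actor or location within a blackboard-set acceptance radius.
; When line of sight is required, an EQS query picks the destination instead.
; Arriving at an actor target finishes with a line-of-sight check as the result.
; Controller-desired rotation follows a task setting during the move and is re-enabled on failure, abort or already at goal.
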(event `self.ReceiveExecute`
  (params (OwnerActor :type "Actor Object Reference"))
  (bind _characterref (`self.CharacterRef`))
  (bind _acceptableradius (`self.AcceptableRadius`))
  (bind (_actorvalue _vectorvalue) (`self.GetBlackBoardValue` (`self.TargetKey`)))
  (bind _asbp_basic_enemy_melee_controller (cast `/Game/AI/BasicEnemies/Melee/BP_BasicEnemyMeleeController` OwnerActor)
    (:`then`
      (`|ExecutionSequence`
        (:`then_0`
          (set `self.AcceptableRadius` (`BTFunctionLibrary.GetBlackboardValueAsFloat` (`self.AcceptableRadiusKey`)))
          (if (not (`self.RequireLineOfSight`))
            (if (`KismetSystemLibrary.IsValid` _actorvalue)
              (bind _returnvalue (`AIController.MoveToActor` _asbp_basic_enemy_melee_controller _actorvalue _acceptableradius true true true null true))
              (set `self.Request` _returnvalue)
              (else
                (bind _returnvalue_2 (`AIController.MoveToLocation` _asbp_basic_enemy_melee_controller _vectorvalue _acceptableradius true true false true null true))
                (set `self.Request` _returnvalue_2)))
            (switch `EPathFollowingRequestResult` (`self.Request`) :!label _label
              (:`Failed`
                (`self.FinishExecute` false :!label _label_2)
                (if (`KismetSystemLibrary.IsValid` _characterref) :!label _label_3
                  (set `CharacterMovementComponent.bUseControllerDesiredRotation` true (`Character.CharacterMovement` _characterref))))
              (:`AlreadyAtGoal`
                (`self.FinishExecute` true)
                (goto _label_3))
              (:`RequestSuccessful`
                (add `AIController.ReceiveMoveCompleted` _asbp_basic_enemy_melee_controller (delegate `ReceiveMoveCompleted`))))
            (else
              (bind _returnvalue_3 (`EnvQueryManager.RunEQSQuery` "/Game/AI/BasicEnemies/Melee/EQS_LineOfSight.EQS_LineOfSight" _asbp_basic_enemy_melee_controller "SingleResult"))
              (`EnvQueryInstanceBlueprintWrapper.SetNamedParam` _returnvalue_3 "Range" (`self.AcceptableRadius`))
              (add `EnvQueryInstanceBlueprintWrapper.OnQueryFinishedEvent` _returnvalue_3 (delegate `OnQueryFinished`)))))
        (:`then_1`
          (bind _ascharacter (cast `Character` (`Controller.K2_GetPawn` _asbp_basic_enemy_melee_controller)))
          (set `self.CharacterRef` _ascharacter)
          (set `CharacterMovementComponent.bUseControllerDesiredRotation` (`self.UseControllerRotation`) (`Character.CharacterMovement` _ascharacter)))))
    (:`CastFailed`
      (goto _label_2))))

(event `ReceiveMoveCompleted`
  (params (RequestID :type "AIRequestID Structure") (Result :type "EPathFollowingResult Enum"))
  (bind _actorvalue (`self.GetBlackBoardValue` (`self.TargetKey`)))
  (switch `EPathFollowingResult` Result
    (:`Success`
      (`/Engine/EditorBlueprintResources/StandardMacros.IsValid` _actorvalue
        (:`Is Valid`
          (`self.FinishExecute` (`Controller.LineOfSightTo` (`Pawn.GetController` (`self.CharacterRef`)) _actorvalue (0.0 0.0 0.0) false)))))
    (:`Blocked`
      (`self.FinishExecute` false :!label _label_4)
      (goto _label_3))
    (:`OffPath`
      (goto _label_4))
    (:`Aborted`
      (goto _label_4))
    (:`Invalid`
      (goto _label_4))))

(event `self.ReceiveAbort`
  (params (OwnerActor :type "Actor Object Reference"))
  (bind _characterref (`self.CharacterRef`))
  (if (`KismetSystemLibrary.IsValid` _characterref)
    (set `CharacterMovementComponent.bUseControllerDesiredRotation` true (`Character.CharacterMovement` _characterref)))
  (`self.FinishAbort`))

(event `OnQueryFinished`
  (params (QueryInstance :type "EnvQueryInstanceBlueprintWrapper Object Reference") (QueryStatus :type "EEnvQueryStatus Enum"))
  (if (`KismetSystemLibrary.IsValid` (stale `self.ReceiveExecute` _asbp_basic_enemy_melee_controller))
    (bind _returnvalue (`AIController.MoveToLocation` (stale `self.ReceiveExecute` _asbp_basic_enemy_melee_controller) (`KismetArrayLibrary.Array_Get` (`EnvQueryInstanceBlueprintWrapper.GetResultsAsLocations` QueryInstance)) 25.0 true true false true null true))
    (set `self.Request` _returnvalue)
    (goto _label)
    (else
      (`self.FinishExecute` false))))

(fn `GetBlackBoardValue`
  (params (Key :type "BlackboardKeySelector Structure"))
  (returns (ActorValue :type "Actor Object Reference") (VectorValue :type "Vector Structure"))
  (if (`KismetSystemLibrary.IsValid` (`BTFunctionLibrary.GetBlackboardValueAsActor` Key))
    (return (`BTFunctionLibrary.GetBlackboardValueAsActor` Key) (0.0 0.0 0.0))
    (else
      (return null (`BTFunctionLibrary.GetBlackboardValueAsVector` Key)))))