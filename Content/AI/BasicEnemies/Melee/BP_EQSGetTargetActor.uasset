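; An EQS context for melee basic enemy AI that supplies the querier's current target actor to environment queries.
; ProvideSingleActor gets the querier's AI controller and reads the TargetActor key from its Blackboard, cast to Actor.
; It returns no actor when the controller or Blackboard is invalid or the cast fails.
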(fn `ProvideSingleActor`
  (params (QuerierObject :type "Object Object Reference") (QuerierActor :type "Actor Object Reference"))
  (returns (ResultingActor :type "Actor Object Reference"))
  (bind _returnvalue (`AIBlueprintHelperLibrary.GetAIController` QuerierActor))
  (if (`KismetSystemLibrary.IsValid` _returnvalue)
    (bind _blackboard (`AIController.Blackboard` _returnvalue))
    (if (`KismetSystemLibrary.IsValid` _blackboard)
      (bind _asactor (cast `Actor` (`BlackboardComponent.GetValueAsObject` _blackboard "TargetActor"))
        (:`then`
          (return _asactor))
        (:`CastFailed`
          _))))
  (return null))