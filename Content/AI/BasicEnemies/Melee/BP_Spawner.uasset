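; BP_Spawner is a box-area enemy spawner that keeps the world topped up to 15 Enemy actors.
; A self-repeating five-second loop refills the shortfall when both the live Enemy count and the BP_EnemyStorage list are under the cap.
; Random ActorsToSpawn classes appear within scaled half-Extent bounds computed in the construction script.
; With OverrideBehavior on, spawns get NewBehavior through their BehaviorComponent, and only these are registered in storage.
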(event `self.ReceiveBeginPlay`
  (bind _outactors (`GameplayStatics.GetAllActorsOfClass` "/Game/AI/BP_EnemyStorage.BP_EnemyStorage_C"))
  (set `self.Storage Ref` (`KismetArrayLibrary.Array_Get` _outactors))
  (`self.SpawnLoop`))

(event `SpawnLoop`
  (`KismetSystemLibrary.Delay` 5.0)
  (`self.Spawn`)
  (`self.SpawnLoop`))

(fn `Spawn`
  (bind _actorstospawn (`self.ActorsToSpawn`))
  (bind _outactors (`GameplayStatics.GetAllActorsOfClass` "/Script/BathrobeSamurai.Enemy"))
  (bind _returnvalue (`KismetArrayLibrary.Array_Length` _outactors))
  (if (and (< _returnvalue 15) (< (`KismetArrayLibrary.Array_Length` (`EnemyStorage.EnemyList` (`self.Storage Ref`))) 15))
    (set `self.NumberOfActors` (- 15 _returnvalue))
    (for _ (range (`self.NumberOfActors`))
      (bind _returnvalue_2 (`|SpawnActorFromClass` (`KismetArrayLibrary.Array_Get` _actorstospawn (`KismetMathLibrary.RandomIntegerInRange` 0 (- (`KismetArrayLibrary.Array_Length` _actorstospawn) 1))) (`KismetMathLibrary.MakeTransform` (+ (`KismetMathLibrary.MakeVector` (`KismetMathLibrary.RandomFloatInRange` (`self.MinX`) (`self.MaxX`)) (`KismetMathLibrary.RandomFloatInRange` (`self.MinY`) (`self.MaxY`)) (`KismetMathLibrary.RandomFloatInRange` (`self.MinZ`) (`self.MaxZ`))) (`self.K2_GetActorLocation`))) "AdjustIfPossibleButAlwaysSpawn" "OverrideRootScale"))
      (if (`self.OverrideBehavior`)
        (bind _item (`KismetArrayLibrary.Array_Get` (`self.K2_GetComponentsByClass` _returnvalue_2 "/Script/BathrobeSamurai.BehaviorComponent")))
        (if (`KismetSystemLibrary.IsValid` _item)
          (`BehaviorComponent.ChangeBehavior` _item (`self.NewBehavior`))
          (bind _asenemy (cast `Enemy` _returnvalue_2))
          (`EnemyStorage.AddEnemyToList` (`self.Storage Ref`) _asenemy))))
    (return)
    (else
      (return))))

(fn `UserConstructionScript`
  (bind _returnvalue (/ (.z (* (`self.Extent`) (`self.GetActorScale3D`))) 2.0))
  (bind _returnvalue_2 (/ (.x (* (`self.Extent`) (`self.GetActorScale3D`))) 2.0))
  (bind _returnvalue_3 (/ (.y (* (`self.Extent`) (`self.GetActorScale3D`))) 2.0))
  (`BoxComponent.SetBoxExtent` (`self.Box`) (`self.Extent`) true)
  (set `self.MinX` (* _returnvalue_2 -1.0))
  (set `self.MaxX` _returnvalue_2)
  (set `self.MinY` (* _returnvalue_3 -1.0))
  (set `self.MaxY` _returnvalue_3)
  (set `self.MinZ` (* _returnvalue -1.0))
  (set `self.MaxZ` _returnvalue))